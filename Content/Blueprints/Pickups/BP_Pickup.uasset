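; BP_Pickup is a generic pickup actor with a spinning mesh and a sphere that detects the first-person character.
; Tick yaws the mesh at a steady rate, then resets its world pitch and roll so it stays upright.
; Sphere overlaps are filtered to FirstPersonCharacter and forwarded to PickupSphereEntered and PickupSphereLeft, which are empty here.
; A hit on the sphere turns on its physics simulation.
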(event OnComponentHit(PickupSphere)
  (params (HitComponent :type Primitive%20Component%20Object%20Reference) (OtherActor :type Actor%20Object%20Reference) (OtherComp :type Primitive%20Component%20Object%20Reference) (NormalImpulse :type Vector :default "0, 0, 0") (Hit :type Hit%20Result%20Structure%20%28by%20ref%29))
  (Physics|SetSimulatePhysics (Variables|Default|GetPickupSphere) true))

(event OnComponentBeginOverlap(PickupSphere)
  (params (OverlappedComponent :type Primitive%20Component%20Object%20Reference) (OtherActor :type Actor%20Object%20Reference) (OtherComp :type Primitive%20Component%20Object%20Reference) (OtherBodyIndex :type Integer) (bFromSweep :type Boolean) (SweepResult :type Hit%20Result%20Structure%20%28by%20ref%29))
  (bind _asfirst_person_character (Utilities|Casting|CastToFirstPersonCharacter OtherActor))
  (CallFunction|PickupSphereEntered _asfirst_person_character))

(event OnComponentEndOverlap(PickupSphere)
  (params (OverlappedComponent :type Primitive%20Component%20Object%20Reference) (OtherActor :type Actor%20Object%20Reference) (OtherComp :type Primitive%20Component%20Object%20Reference) (OtherBodyIndex :type Integer))
  (bind _asfirst_person_character (Utilities|Casting|CastToFirstPersonCharacter OtherActor))
  (CallFunction|PickupSphereLeft _asfirst_person_character))

(event Custom|PickupSphere%20Entered
  (params (Character :type First%20Person%20Character%20Object%20Reference)))

(event Custom|PickupSphere%20Left
  (params (Character :type First%20Person%20Character%20Object%20Reference)))

(event EventTick
  (params (DeltaSeconds :type Float%20%28single-precision%29))
  (bind _pickupmesh (Variables|Default|GetPickupMesh))
  ;[0.07994 1 0.2806 1 22] Make Pick up rotate maintaining upward World rotation
  (Transformation|AddRelativeRotation _pickupmesh (Math|Rotator|MakeRotator 0.0 0.0 (* DeltaSeconds 1.8e+02)) false false)
  (Transformation|SetWorldRotation (Variables|Default|GetPickupMesh) (Math|Rotator|MakeRotator 0.0 0.0 (.Yaw (Math|Rotator|BreakRotator (Transformation|GetWorldRotation _pickupmesh)))) false false))

(fn ConstructionScript)