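; BP_HealthPickup is a pickup that restores health to a character entering its sphere.
; It handles the sphere-entered event only on the authority, applying the pickup and destroying itself only if the character is below max health.
; It passes HealthToGive negated to the character's ModifyHealth.
; The construction script only calls the parent's.
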(event EventPickupSphereEntered
  (params (Character :type First%20Person%20Character%20Object%20Reference))
  (Networking|SwitchHasAuthority
    (:Authority
      (if (< (Variables|/Game/FirstPersonBP/Blueprints/FirstPersonCharacter.FirstPersonCharacter_C|GetHealth Character) (Variables|/Game/FirstPersonBP/Blueprints/FirstPersonCharacter.FirstPersonCharacter_C|GetMax_Health Character))
        (Default|ModifyHealth Character (* (Variables|Default|GetHealthToGive) -1.0))
        (Actor|DestroyActor)))))

(fn ConstructionScript
  (|CallParentFunction))