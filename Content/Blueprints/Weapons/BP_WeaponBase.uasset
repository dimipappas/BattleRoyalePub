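; Base weapon Blueprint that tracks clip and spare ammo for a FirstPersonCharacter owner, cached on the server at BeginPlay.
; GunFired spends ammo on authority, throttled by the owner's Firing flag and a short delay, and triggers a timed Reload on empty.
; Reload refills the clip from spare ammo while flagging the owner as Reloading.
; The authority-only giveammo tops up the clip but zeroes spare ammo on overflow, as the capped-addition expression is unconnected.
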(event Custom|give%20ammo
  (params (ammo%20to%20give :type Integer))
  ;[0 1 0.05499] event to give ammo
  (Networking|SwitchHasAuthority
    (:Authority
      (Variables|ammo|SetCurrentAmmo (+ (Variables|ammo|GetCurrentAmmo) (Math|Integer|Min(Integer) ammo%20to%20give (- (Variables|ammo|GetClipSize) (Variables|ammo|GetCurrentAmmo)))))
      (if (> (- ammo%20to%20give (Math|Integer|Min(Integer) ammo%20to%20give (- (Variables|ammo|GetClipSize) (Variables|ammo|GetCurrentAmmo)))) 0)
        (Variables|ammo|SetCurrentSpareAmmo 0)))))

(event Custom|Gun%20Fired
  (bind _current_owner (Variables|Default|Getcurrent%20owner))
  (bind _currentammo (Variables|ammo|GetCurrentAmmo))
  ;[1 1 1] When gun is fired, take ammo and reload if necessary
  (Networking|SwitchHasAuthority
    (:Authority
      (if (not (Variables|/Game/FirstPersonBP/Blueprints/FirstPersonCharacter.FirstPersonCharacter_C|GetFiring? (Variables|Default|Getcurrent%20owner)))
        (Math|Integer|DecrementInt _currentammo
          (:%20%20
            (if (<= _currentammo 0)
              (CallFunction|Reload)
              (else
                (Variables|/Game/FirstPersonBP/Blueprints/FirstPersonCharacter.FirstPersonCharacter_C|SetFiring? _current_owner true)
                (Utilities|FlowControl|Delay 0.2)
                (Variables|/Game/FirstPersonBP/Blueprints/FirstPersonCharacter.FirstPersonCharacter_C|SetFiring? _current_owner false)))))))))

(event Custom|Reload
  ;[1 1 1] Reload Event
  (Variables|/Game/FirstPersonBP/Blueprints/FirstPersonCharacter.FirstPersonCharacter_C|SetReloading? (Variables|Default|Getcurrent%20owner) true)
  (Utilities|FlowControl|Delay 2.0)
  (Variables|ammo|SetCurrentAmmo (Math|Integer|Min(Integer) (Variables|ammo|GetCurrentSpareAmmo) (Variables|ammo|GetClipSize)))
  (Variables|ammo|SetCurrentSpareAmmo (Math|Integer|Max(Integer) (- (Variables|ammo|GetCurrentSpareAmmo) (Math|Integer|Min(Integer) (Variables|ammo|GetCurrentSpareAmmo) (Variables|ammo|GetClipSize)))))
  (Variables|/Game/FirstPersonBP/Blueprints/FirstPersonCharacter.FirstPersonCharacter_C|SetReloading? (Variables|Default|Getcurrent%20owner) false))

(event EventBeginPlay
  ;[1 0 0.01801] On begin play setup our ammo ammount
  (Networking|SwitchHasAuthority
    (:Authority
      (Variables|ammo|SetCurrentAmmo (Variables|ammo|GetClipSize))
      (Variables|ammo|SetCurrentSpareAmmo (Variables|ammo|GetStartingSpareAmmo))
      (bind _asfirst_person_character (Utilities|Casting|CastToFirstPersonCharacter (Components|GetOwner)))
      (Variables|Default|Setcurrent%20owner _asfirst_person_character))))

(fn ConstructionScript)

(fn HasAmmo?
  (return (> (Variables|ammo|GetCurrentAmmo) 0)))